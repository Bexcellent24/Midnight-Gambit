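; Arcade machine the player can use once, playable only when the level counter passed to it is a multiple of three.
; Box overlap shows a working or out-of-order prompt and gates the Interact input, which opens the arcade widget with mouse cursor.
; It also stores the level's stairs; RemoveStairs destroys a random stair's button, re-rolling recursively to spare the up stairs.
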(event `self.ReceiveBeginPlay`
  (`self.EnableInput` (`GameplayStatics.GetPlayerController` 0))
  (bind _asbp_game_instance (cast `/Game/Blueprints/BP_GameInstance` (`GameplayStatics.GetGameInstance`)))
  (`/Game/Blueprints/BP_GameInstance.CheckIfLevel3` _asbp_game_instance))

(event `EnhancedInput|/Game/FirstPerson/Input/Actions/IA_Interact`
  (params (ActionValue :type Boolean) (ElapsedSeconds :type "Float (double-precision)") (TriggeredSeconds :type "Float (double-precision)") (InputAction :type "InputAction Object Reference" :default "/Game/FirstPerson/Input/Actions/IA_Interact.IA_Interact"))
  (bind _returnvalue (`GameplayStatics.GetPlayerController` 0))
  (bind _canplay (`self.CanPlay`))
  (:`Started`
    (if (not (`self.PlayedGame`))
      (`/Engine/EditorBlueprintResources/StandardMacros.Gate` true :!label _label
        (:`Exit`
          (`/Engine/EditorBlueprintResources/StandardMacros.IsValid` (stale `self.Box.OnComponentBeginOverlap` _returnvalue)
            (:`Is Valid`
              (`Widget.RemoveFromParent` (stale `self.Box.OnComponentBeginOverlap` _returnvalue))
              (set `self.PlayedGame` true)
              (`KismetSystemLibrary.PrintString` (`KismetStringLibrary.Concat_StrStr` "Can Play" (`KismetStringLibrary.Conv_BoolToString` _canplay)))
              (if _canplay
                (bind _returnvalue_2 (`|CreateWidget` "/Game/UI/WB_Archade.WB_Archade_C"))
                (`UserWidget.AddToViewport` _returnvalue_2 0)
                (set `PlayerController.bShowMouseCursor` true _returnvalue)
                (`WidgetBlueprintLibrary.SetInputMode_GameAndUIEx` _returnvalue _returnvalue_2)))))))))

(event `self.Box.OnComponentBeginOverlap`
  (params (OverlappedComponent :type "PrimitiveComponent Object Reference") (OtherActor :type "Actor Object Reference") (OtherComp :type "PrimitiveComponent Object Reference") (OtherBodyIndex :type Integer) (bFromSweep :type Boolean) (SweepResult :type "HitResult Structure (by ref)"))
  (cast `/Game/Blueprints/BP_FirstPersonCharacter` OtherActor)
  (if (`self.CanPlay`)
    (if (not (`self.PlayedGame`))
      (bind _returnvalue (`|CreateWidget` "/Game/UI/WB_Working.WB_Working_C"))
      (`UserWidget.AddToViewport` _returnvalue 0)
      (goto _label :!via `Open`))
    (else
      (bind _returnvalue_2 (`|CreateWidget` "/Game/UI/WB_OutOfOrder.WB_OutOfOrder_C"))
      (`UserWidget.AddToViewport` _returnvalue_2 0))))

(event `self.Box.OnComponentEndOverlap`
  (params (OverlappedComponent :type "PrimitiveComponent Object Reference") (OtherActor :type "Actor Object Reference") (OtherComp :type "PrimitiveComponent Object Reference") (OtherBodyIndex :type Integer))
  (cast `/Game/Blueprints/BP_FirstPersonCharacter` OtherActor)
  (if (`self.CanPlay`)
    (`/Engine/EditorBlueprintResources/StandardMacros.IsValid` (stale `self.Box.OnComponentBeginOverlap` _returnvalue)
      (:`Is Valid`
        (`Widget.RemoveFromParent` (stale `self.Box.OnComponentBeginOverlap` _returnvalue))
        (goto _label :!via `Close`)))
    (else
      (`Widget.RemoveFromParent` (stale `self.Box.OnComponentBeginOverlap` _returnvalue_2)))))

(event `GetStairs`
  (params (Stairs :type "Array of /Game/Blueprints/BP_Stairs Object Reference") (UpStairsIndex :type Integer))
  (`KismetSystemLibrary.PrintString` (`KismetStringLibrary.Concat_StrStr` (`KismetStringLibrary.Conv_IntToString` (`KismetArrayLibrary.Array_Length` Stairs)) (`KismetStringLibrary.Conv_IntToString` UpStairsIndex)))
  (set `self.Stairs` Stairs)
  (set `self.UpSairsIndex` UpStairsIndex))

(event `RemoveStairs`
  (`self.ChooseBadDoor`)
  (`KismetSystemLibrary.Delay` 0.5)
  (`KismetSystemLibrary.PrintString` (`KismetStringLibrary.Concat_StrStr` "Bad Egg: " (`KismetStringLibrary.Conv_IntToString` (`self.BadEggDoor`))) true true (struct :`R` 0.956059 :`B` 1.0 :`A` 1.0) 10.0)
  (`KismetSystemLibrary.PrintString` (`KismetStringLibrary.Concat_StrStr` "Up stairs: " (`KismetStringLibrary.Conv_IntToString` (`self.UpSairsIndex`))) true true (struct :`R` 0.956059 :`B` 1.0 :`A` 1.0) 10.0)
  (`self.K2_DestroyActor` (`/Game/Blueprints/BP_Stairs.StairButton` (`|GetArrayItem` (`self.Stairs`) (`self.BadEggDoor`)))))

(event `ChooseBadDoor`
  (bind _output_get (set `self.BadEggDoor` (`KismetMathLibrary.RandomIntegerInRange` 0 (- (`KismetArrayLibrary.Array_Length` (`self.Stairs`)) 1))))
  (if (not (!= _output_get (`self.UpSairsIndex`)))
    (`self.ChooseBadDoor`)))

(event `CheckIfAchadeLevel`
  (params (Tick :type Integer))
  (if (== (mod Tick 3) 0)
    (bind _output_get (set `self.CanPlay` true))
    (`KismetSystemLibrary.PrintString` (`KismetStringLibrary.Conv_BoolToString` _output_get) true true (struct :`G` 1.0 :`B` 0.554045 :`A` 1.0) 3.0)))

(fn `UserConstructionScript`)