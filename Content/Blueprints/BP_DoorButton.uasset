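; Interactable door button that sends an interact message to its target door once the podium's souls are paid.
; A box overlap opens and closes a gate so the interact input only registers while the first-person character is nearby.
; A pressed flag on the character blocks further presses.
; A successful press plays a click and timelines that lerp the button in and back out.
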(event `self.ReceiveBeginPlay`
  (bind (_returnvalue_location _returnvalue_rotation _returnvalue_scale) (`KismetMathLibrary.BreakTransform` (`SceneComponent.GetRelativeTransform` (`self.Button`))))
  (set `self.OutPos` (`KismetMathLibrary.MakeTransform` _returnvalue_location _returnvalue_rotation _returnvalue_scale))
  (set `self.InPos` (`KismetMathLibrary.MakeTransform` (- _returnvalue_location (0.0 0.0 10.0)) _returnvalue_rotation _returnvalue_scale))
  (`self.EnableInput` (`GameplayStatics.GetPlayerController` 0))
  (bind _returnvalue (`GameplayStatics.GetActorOfClass` "/Game/Blueprints/BP_Podium.BP_Podium_C"))
  (set `self.PodiumRef` _returnvalue))

(event `EnhancedInput|/Game/FirstPerson/Input/Actions/IA_Interact`
  (params (ActionValue :type Boolean) (ElapsedSeconds :type "Float (double-precision)") (TriggeredSeconds :type "Float (double-precision)") (InputAction :type "InputAction Object Reference" :default "/Game/FirstPerson/Input/Actions/IA_Interact.IA_Interact"))
  (bind _targetdoor (`self.TargetDoor`))
  ;[1 1 1] Button Interaction (Push Button)
  (:`Started`
    (`/Engine/EditorBlueprintResources/StandardMacros.Gate` true :!label _label
      (:`Exit`
        (if (`/Game/Blueprints/BP_FirstPersonCharacter.HasPressedButton` (stale `self.Box.OnComponentBeginOverlap` _output_get))
          _
          (elif (`/Game/Blueprints/BP_Podium.SoulsPaid` (`self.PodiumRef`))
            (if (`KismetSystemLibrary.DoesImplementInterface` _targetdoor "/Game/Interfaces/InteractInterface.InteractInterface_C")
              (message `/Game/Interfaces/InteractInterface.Interact` _targetdoor)
              (set `/Game/Blueprints/BP_FirstPersonCharacter.HasPressedButton` true (`self.As BP First Person Character`))
              (`GameplayStatics.PlaySoundAtLocation` "/Game/Audio/Button_Click.Button_Click" (`self.K2_GetActorLocation`) (struct) 1.0 1.0 0.0 null null null null)
              (bind (_direction _button_in) (`Timeline|Button In` :!via `PlayFromStart`)
                (:`Update`
                  (`SceneComponent.K2_SetRelativeTransform` (`self.Button`) (`KismetMathLibrary.TLerp` (`self.OutPos`) (`self.InPos`) _button_in) false false))
                (:`Finished`
                  (bind (_direction_2 _button_in_2) (`Timeline|Button Out` :!via `ReverseFromEnd`)
                    (:`Update`
                      (`SceneComponent.K2_SetRelativeTransform` (`self.Button`) (`KismetMathLibrary.TLerp` (`self.OutPos`) (`self.InPos`) _button_in_2) false false))))))))))))

(event `self.Box.OnComponentBeginOverlap`
  (params (OverlappedComponent :type "PrimitiveComponent Object Reference") (OtherActor :type "Actor Object Reference") (OtherComp :type "PrimitiveComponent Object Reference") (OtherBodyIndex :type Integer) (bFromSweep :type Boolean) (SweepResult :type "HitResult Structure (by ref)"))
  ;[1 1 1] Button Interaction (Push Button)
  (bind _asbp_first_person_character (cast `/Game/Blueprints/BP_FirstPersonCharacter` OtherActor))
  (bind _output_get (set `self.As BP First Person Character` _asbp_first_person_character))
  (goto _label :!via `Open`))

(event `self.Box.OnComponentEndOverlap`
  (params (OverlappedComponent :type "PrimitiveComponent Object Reference") (OtherActor :type "Actor Object Reference") (OtherComp :type "PrimitiveComponent Object Reference") (OtherBodyIndex :type Integer))
  ;[1 1 1] Button Interaction (Push Button)
  (cast `/Game/Blueprints/BP_FirstPersonCharacter` OtherActor)
  (goto _label :!via `Close`))

(fn `UserConstructionScript`)