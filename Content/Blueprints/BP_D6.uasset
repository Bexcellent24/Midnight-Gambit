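; Physics-driven six-sided die actor that rolls and reports its result to the first-person character.
; RollDIce enables simulation, applies a fixed impulse at the die's location, then freezes it after a fixed delay.
; Result finds the face up by comparing six arrow components' forward vectors to world up with a tolerance.
; It then updates the linked widget, passes the roll to the character, and after a pause closes the widget and restores game-only input.
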(event `RollDIce`
  (bind _d6 (`self.D6`))
  (`PrimitiveComponent.SetSimulatePhysics` (`self.D6`) true)
  (`PrimitiveComponent.AddImpulseAtLocation` _d6 (20000.0 20000.0 20000.0) (`SceneComponent.K2_GetComponentLocation` _d6) "None")
  (`KismetSystemLibrary.Delay` 3.0)
  (`PrimitiveComponent.SetSimulatePhysics` (`self.D6`) false)
  (`self.Result`))

(event `Stopped`
  (if (`SceneComponent.IsSimulatingPhysics` (`self.D6`) "None")
    (`self.Stopped`)
    (else
      (`self.Result`)
      (`PrimitiveComponent.SetSimulatePhysics` (`self.D6`) true))))

(event `Result`
  (bind _returnvalue (`GameplayStatics.GetPlayerController` 0))
  (if (== (`SceneComponent.GetForwardVector` (`self.Arrow1`)) (0.0 0.0 1.0) :`ErrorTolerance` 0.5)
    (set `self.RollResult` 1)
    (`KismetSystemLibrary.PrintString` "1")
    (`/Game/UI/WB_D6.UpdateText` (`self.Widget`) :!label _label)
    (bind _asbp_first_person_character (cast `/Game/Blueprints/BP_FirstPersonCharacter` (`GameplayStatics.GetPlayerCharacter` 0)))
    (`/Game/Blueprints/BP_FirstPersonCharacter.GetRollResult` _asbp_first_person_character (`self.RollResult`))
    (`KismetSystemLibrary.Delay` 1.5)
    (`Widget.RemoveFromParent` (`self.Widget`))
    (`WidgetBlueprintLibrary.SetInputMode_GameOnly` _returnvalue)
    (set `PlayerController.bShowMouseCursor` false _returnvalue)
    (elif (== (`SceneComponent.GetForwardVector` (`self.Arrow2`)) (0.0 0.0 1.0) :`ErrorTolerance` 0.5)
      (set `self.RollResult` 2)
      (`KismetSystemLibrary.PrintString` "2")
      (goto _label)
      (elif (== (`SceneComponent.GetForwardVector` (`self.Arrow3`)) (0.0 0.0 1.0) :`ErrorTolerance` 0.5)
        (set `self.RollResult` 3)
        (`KismetSystemLibrary.PrintString` "3")
        (goto _label)
        (elif (== (`SceneComponent.GetForwardVector` (`self.Arrow4`)) (0.0 0.0 1.0) :`ErrorTolerance` 0.5)
          (set `self.RollResult` 4)
          (`KismetSystemLibrary.PrintString` "4")
          (goto _label)
          (elif (== (`SceneComponent.GetForwardVector` (`self.Arrow5`)) (0.0 0.0 1.0) :`ErrorTolerance` 0.5)
            (set `self.RollResult` 5)
            (`KismetSystemLibrary.PrintString` "5")
            (goto _label)
            (elif (== (`SceneComponent.GetForwardVector` (`self.Arrow6`)) (0.0 0.0 1.0) :`ErrorTolerance` 0.5)
              (set `self.RollResult` 6)
              (`KismetSystemLibrary.PrintString` "6")
              (goto _label))))))))

(event `SetD6Refernce`
  (params (Widget :type "/Game/UI/WB_D6 Object Reference"))
  (set `self.Widget` Widget))

(fn `UserConstructionScript`)