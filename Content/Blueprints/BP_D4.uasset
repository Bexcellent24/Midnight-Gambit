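; A four-sided die Blueprint that rolls with physics and reports the result to the first-person character.
; RollDIce applies an impulse, waits a fixed delay, then freezes the die and calls Result.
; Result finds which of four arrow components points near world up, updates the widget and passes the number to the character.
; After a short pause it removes the widget and restores game-only input with a hidden cursor.
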(event `RollDIce`
  (bind _d4 (`self.D4`))
  (`PrimitiveComponent.SetSimulatePhysics` (`self.D4`) true)
  (`PrimitiveComponent.AddImpulseAtLocation` _d4 (2000.0 2000.0 2000.0) (`SceneComponent.K2_GetComponentLocation` _d4) "None")
  (`KismetSystemLibrary.Delay` 4.0)
  (`PrimitiveComponent.SetSimulatePhysics` (`self.D4`) false)
  (`PrimitiveComponent.SetEnableGravity` _d4 true)
  (`self.Result`))

(event `Stopped`
  (if (`SceneComponent.IsSimulatingPhysics` (`self.D4`) "None")
    (`self.Stopped`)
    (else
      (`self.Result`)
      (`PrimitiveComponent.SetSimulatePhysics` (`self.D4`) true))))

(event `Result`
  (bind _returnvalue (`GameplayStatics.GetPlayerController` 0))
  (if (== (`SceneComponent.GetForwardVector` (`self.Arrow1`)) (0.0 0.0 1.0) :`ErrorTolerance` 0.5)
    (set `self.RollResult` 1)
    (`/Game/UI/WB_D4.UpdateText` (`self.Widget`) :!label _label)
    (bind _asbp_first_person_character (cast `/Game/Blueprints/BP_FirstPersonCharacter` (`GameplayStatics.GetPlayerCharacter` 0)))
    (`/Game/Blueprints/BP_FirstPersonCharacter.GetRollResult` _asbp_first_person_character (`self.RollResult`))
    (`KismetSystemLibrary.Delay` 1.5)
    (`Widget.RemoveFromParent` (`self.Widget`))
    (`WidgetBlueprintLibrary.SetInputMode_GameOnly` _returnvalue)
    (set `PlayerController.bShowMouseCursor` false _returnvalue)
    (elif (== (`SceneComponent.GetForwardVector` (`self.Arrow2`)) (0.0 0.0 1.0) :`ErrorTolerance` 0.5)
      (set `self.RollResult` 2)
      (goto _label)
      (elif (== (`SceneComponent.GetForwardVector` (`self.Arrow3`)) (0.0 0.0 1.0) :`ErrorTolerance` 0.5)
        (set `self.RollResult` 3)
        (goto _label)
        (elif (== (`SceneComponent.GetForwardVector` (`self.Arrow4`)) (0.0 0.0 1.0) :`ErrorTolerance` 0.5)
          (set `self.RollResult` 4)
          (goto _label))))))

(event `SetD4Refernce`
  (params (Widget :type "/Game/UI/WB_D4 Object Reference"))
  (set `self.Widget` Widget))

(fn `UserConstructionScript`)