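; BP_Podium is an interactable podium that shows the WB_Podium UI while something overlaps its Box trigger, as long as SoulsPaid is false.
; Begin overlap creates the widget, shows the mouse cursor and switches to Game and UI input.
; End overlap removes it and restores game-only input.
; The overlap events do not filter by actor, and SoulsPaid is only read here.
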(event `CloseWidget`
  (bind _returnvalue (`GameplayStatics.GetPlayerController` 0))
  (bind _podiumwidget (`self.PodiumWidget`))
  (`/Engine/EditorBlueprintResources/StandardMacros.IsValid` _podiumwidget
    (:`Is Valid`
      (`Widget.RemoveFromParent` _podiumwidget)
      (set `PlayerController.bShowMouseCursor` false _returnvalue)
      (`WidgetBlueprintLibrary.SetInputMode_GameOnly` _returnvalue))))

(event `OpenWidget`
  (bind _returnvalue (`GameplayStatics.GetPlayerController` 0))
  (bind _returnvalue_2 (`|CreateWidget` "/Game/UI/WB_Podium.WB_Podium_C" null null))
  (bind _output_get (set `self.PodiumWidget` _returnvalue_2))
  (`UserWidget.AddToViewport` _returnvalue_2 0)
  (`UserWidget.AddToViewport` _output_get 0)
  (set `PlayerController.bShowMouseCursor` true _returnvalue)
  (`WidgetBlueprintLibrary.SetInputMode_GameAndUIEx` _returnvalue (`self.PodiumWidget`)))

(event `self.Box.OnComponentBeginOverlap`
  (params (OverlappedComponent :type "PrimitiveComponent Object Reference") (OtherActor :type "Actor Object Reference") (OtherComp :type "PrimitiveComponent Object Reference") (OtherBodyIndex :type Integer) (bFromSweep :type Boolean) (SweepResult :type "HitResult Structure (by ref)"))
  (if (not (`self.SoulsPaid`))
    (`self.OpenWidget`)))

(event `self.Box.OnComponentEndOverlap`
  (params (OverlappedComponent :type "PrimitiveComponent Object Reference") (OtherActor :type "Actor Object Reference") (OtherComp :type "PrimitiveComponent Object Reference") (OtherBodyIndex :type Integer))
  (`self.CloseWidget`))

(fn `UserConstructionScript`)