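; BP_Stairs is a stairs actor that moves the player between levels through separate up and down overlap boxes.
; When a BP_FirstPersonCharacter enters either box, it shows a WB_LevelFade widget and waits briefly.
; It then calls GoUpLevel or GoDownLevel on BP_GameInstance, and both paths continue to a shared "faild" debug print.
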(event `self.UpBox.OnComponentBeginOverlap`
  (params (OverlappedComponent :type "PrimitiveComponent Object Reference") (OtherActor :type "Actor Object Reference") (OtherComp :type "PrimitiveComponent Object Reference") (OtherBodyIndex :type Integer) (bFromSweep :type Boolean) (SweepResult :type "HitResult Structure (by ref)"))
  (cast `/Game/Blueprints/BP_FirstPersonCharacter` OtherActor)
  (bind _returnvalue (`|CreateWidget` "/Game/UI/WB_LevelFade.WB_LevelFade_C"))
  (`UserWidget.AddToViewport` _returnvalue 0)
  (`/Game/UI/WB_LevelFade.Fadeer` _returnvalue)
  (`KismetSystemLibrary.Delay` 0.5)
  (bind _asbp_game_instance (cast `/Game/Blueprints/BP_GameInstance` (`GameplayStatics.GetGameInstance`)))
  (`/Game/Blueprints/BP_GameInstance.GoUpLevel` _asbp_game_instance)
  (`KismetSystemLibrary.PrintString` "faild" :!label _label))

(event `self.DownBox.OnComponentBeginOverlap`
  (params (OverlappedComponent :type "PrimitiveComponent Object Reference") (OtherActor :type "Actor Object Reference") (OtherComp :type "PrimitiveComponent Object Reference") (OtherBodyIndex :type Integer) (bFromSweep :type Boolean) (SweepResult :type "HitResult Structure (by ref)"))
  (cast `/Game/Blueprints/BP_FirstPersonCharacter` OtherActor)
  (bind _returnvalue (`|CreateWidget` "/Game/UI/WB_LevelFade.WB_LevelFade_C"))
  (`UserWidget.AddToViewport` _returnvalue 0)
  (`/Game/UI/WB_LevelFade.Fadeer` _returnvalue)
  (`KismetSystemLibrary.Delay` 0.5)
  (bind _asbp_game_instance (cast `/Game/Blueprints/BP_GameInstance` (`GameplayStatics.GetGameInstance`)))
  (`/Game/Blueprints/BP_GameInstance.GoDownLevel` _asbp_game_instance)
  (goto _label))

(fn `UserConstructionScript`)